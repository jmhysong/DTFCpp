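; Character Blueprint that gives the player an in-game chat by spawning and owning a Chat_System actor.
; BeginPlay waits briefly for client players to initialize, then, on authority only, calls SpawnChatOnServer to spawn it at the character's location and store the reference.
; Enter focuses the chat input, and Left/Right cycle tabs with wraparound for cursorless play.
; SpawnIt duplicates the spawn logic but is not called in this Blueprint.
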(event Custom|Spawn%20Chat%20on%20Server
  ;[0.1631 1 0.03067] Add this to your character blueprint
  (bind _returnvalue (Game|SpawnActorfromClass "/Game/BPChatSystem/Blueprints/Chat_System.Chat_System_C" (Math|Transform|MakeTransform (Transformation|GetActorLocation) "0, 0, 0" "1.000000,1,1") "Undefined" self "" 0))
  (Variables|Default|SetChat%20System _returnvalue))

(event EventBeginPlay
  ;[0.1631 1 0.03067] Add this to your character blueprint
  ;;[1 1 1] Spawn the chat at the beginning of the game
  (Utilities|FlowControl|Delay 1.0) ; Allow time for the client players to initialize, otherwise things won't work properly
  (Networking|SwitchHasAuthority
    (:Authority
      (CallFunction|SpawnChatonServer))))

(event Input|KeyboardEvents|Left
  (params (Key :type Key%20Structure :default "AnyKey"))
  ;[0.1631 1 0.03067] Add this to your character blueprint
  ;;[0 0.459 0.755] This is used for games where you can't see the mouse cursor but want to change groups/tabs, you can call these functions from anywhere
  (:Pressed
    (Default|Previous/NextTab (Variables|Default|GetChat%20System) "NewEnumerator0" true)))

(event Input|KeyboardEvents|Right
  (params (Key :type Key%20Structure :default "AnyKey"))
  ;[0.1631 1 0.03067] Add this to your character blueprint
  ;;[0 0.459 0.755] This is used for games where you can't see the mouse cursor but want to change groups/tabs, you can call these functions from anywhere
  (:Pressed
    (Default|Previous/NextTab (Variables|Default|GetChat%20System) "NewEnumerator1" true)))

(event Input|KeyboardEvents|Enter
  (params (Key :type Key%20Structure :default "AnyKey"))
  ;[0.1631 1 0.03067] Add this to your character blueprint
  (:Pressed
    (Default|SetKeyboardFocustoChatInput (Variables|Default|GetChat%20System))))

(fn ConstructionScript)

(fn SpawnIt
  (bind _returnvalue (Game|SpawnActorfromClass "/Game/BPChatSystem/Blueprints/Chat_System.Chat_System_C" (Math|Transform|MakeTransform (Transformation|GetActorLocation) "0, 0, 0" "1.000000,1,1") "Undefined" self "" 0))
  (Variables|Default|SetChat%20System _returnvalue))